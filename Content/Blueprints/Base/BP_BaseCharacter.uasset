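; Base character Blueprint that provides health, alive state, a kill counter and physics-driven upper-body animation.
; On BeginPlay it fills Health to MaxHealth through HealthRemove, despite that name, then applies physical animation and simulates physics on bodies from spine_01 down the bone chain.
; Helper functions subtract clamped damage, report alive from the Dead flag and increment kills; nothing here sets Dead.
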(event EventBeginPlay
  ;[0 0 0] BeginPlay
  ;;[0.008078 1 0] Health
  (CallFunction|HealthRemove)
  ;;[1 0.5749 0.1956] Activate Physics
  (CallFunction|ActivatePhysicsAsset (Utilities|Struct|MakePhysicalAnimationData false 1.0 2e+02 1.7e+03 2e+02) "spine_01"))

(fn ConstructionScript)

(fn ActivatePhysicsAsset
  (params (PhysicalAnimationData :type Physical%20Animation%20Data%20Structure%20%28by%20ref%29) (InputPin :type Name))
  (Utilities|FlowControl|Sequence
    (:then_0
      (Class|PhysicalAnimationComponent|SetSkeletalMeshComponent (Variables|Default|GetPhysicalAnimation) (Variables|Character|GetMesh))
      (Class|PhysicalAnimationComponent|ApplyPhysicalAnimationSettingsBelow (Variables|Default|GetPhysicalAnimation) InputPin PhysicalAnimationData true)
      (Class|SkeletalMeshComponent|SetAllBodiesBelowSimulatePhysics (Variables|Character|GetMesh) InputPin true true))))

(fn DeacreamsHealth
  (params (Damage :type Float%20%28single-precision%29))
  (bind _output_get (Variables|Default|SetHealth (Math|Float|Clamp(Float) (- (Variables|Default|GetHealth) Damage) 0.0 (Variables|Default|GetMaxHealth))))
  (return _output_get))

(fn IsAlive
  (return (not (Variables|Default|GetDead))))

(fn IncreaseKill
  (Math|Integer|IncrementInt (Variables|Default|GetKill)))

(fn HealthRemove
  (Variables|Default|SetHealth (Variables|Default|GetMaxHealth)))