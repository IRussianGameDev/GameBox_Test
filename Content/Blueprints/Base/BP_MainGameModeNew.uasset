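; Game mode that creates the player HUD and runs escalating enemy waves until the wave counter reaches three.
; Each wave multiplies the enemy quota, then a looping timer spawns enemies with a particle burst at random TargetPoints until it is spent.
; Random rolls gated by wave number choose Doge, Efirium or Bitcoin AI.
; RegisterEnemyDeath prunes the live enemy array and, once wave completion is met, starts the next wave after a delay.
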(event Custom|SpawnWave
  (CallFunction|SpawnEnemy))

(event Custom|EndWave
  (Utilities|FlowControl|Delay 3.0)
  (if (< (Variables|Default|GetCurrentWave) 3)
    (CallFunction|StartNewWave)))

(event EventBeginPlay
  (Utilities|FlowControl|Sequence
    (:then_1
      (bind _returnvalue (UserInterface|CreateWidget "/Game/UI/W_PlayerHudOrigin.W_PlayerHudOrigin_C"))
      (UserInterface|Viewport|AddtoViewport _returnvalue 0)
      (Utilities|FlowControl|Delay 2.0)
      (CallFunction|StartNewWave))))

(event EventTick
  (params (DeltaSeconds :type Float%20%28single-precision%29)))

(fn ConstructionScript)

(fn StartNewWave
  (Math|Integer|IncrementInt (Variables|Default|GetCurrentWave)
    (:%20%20
      (CallFunction|IncreaseWaveDifficulity)
      (Utilities|Time|SetTimerbyFunctionName 0 "SpawnWave" (Variables|Default|GetTime) true))))

(fn SpawnEnemy
  (bind _spawnpoint (CallFunction|GetRandomSpawnPoint))
  (Utilities|IsValid _spawnpoint
    (:Is%20Valid
      (Effects|SpawnEmitteratLocation "/Game/FX/PS_ExplosionPerl.PS_ExplosionPerl" (Transformation|GetActorLocation _spawnpoint) "0, 0, 0" "0.600000,0.600000,0.600000")
      (bind _output_get (CallFunction|RandomSpawnClass))
      (bind _returnvalue (Game|SpawnActorfromClass _output_get (Transformation|GetActorTransform _spawnpoint) "Undefined" 0 0))
      (Utilities|IsValid _returnvalue
        (:Is%20Valid
          (Utilities|Array|Add (Variables|Default|GetBP_Enemy) _returnvalue)
          (bind _result (Math|Integer|DecrementInt (Variables|Default|GetEnemySpawnRemaining))
            (:%20%20
              (if (== _result 0)
                (Utilities|Time|ClearTimerbyFunctionName 0 "SpawnWave")))))))))

(fn GetRandomSpawnPoint
  (bind _outactors (Actor|GetAllActorsOfClass "/Script/Engine.TargetPoint"))
  (return (Utilities|Array|Get(acopy) _outactors (Math|Random|RandomIntegerinRange 0 (Utilities|Array|LastIndex _outactors)))))

(fn RegisterEnemyDeath
  (params (Enemy :type BP%20AI%20Doge%20Object%20Reference%20%28by%20ref%29))
  (Utilities|Array|RemoveItem (Variables|Default|GetBP_Enemy) Enemy)
  (if (CallFunction|IsWaveComplite)
    (CallFunction|EndWave)))

(fn IsWaveComplite
  (return (and (== (Utilities|Array|Length (Variables|Default|GetBP_Enemy)) 0) (== (Variables|Default|GetEnemySpawnRemaining) 0))))

(fn IncreaseWaveDifficulity
  (bind _output_get (Variables|Default|SetWaveDiffculity (Math|Float|Round (* (Variables|Default|GetWaveDiffculity) (Variables|Default|GetDiffculityMultiplier)))))
  (Variables|Default|SetEnemySpawnRemaining _output_get))

(fn RandomSpawnClass
  (bind _returnvalue (Math|Random|RandomFloatinRange 0.0 1.0))
  (bind _currentwave (Variables|Default|GetCurrentWave))
  (if (<= _returnvalue 0.33)
    (if true
      (bind _output_get (Variables|Default|SetClass "/Game/Blueprints/Base/BP_AIDoge.BP_AIDoge_C"))
      (return _output_get))
    (elif (and (> _returnvalue 0.33) (<= _returnvalue 0.66))
      (if (and (> _currentwave 1) (< _currentwave 3))
        (bind _output_get_2 (Variables|Default|SetClass "/Game/Blueprints/Base/BP_AIEfirium.BP_AIEfirium_C"))
        (return _output_get_2))
      (elif (and (> _returnvalue 0.9) (>= _currentwave 3))
        (bind _output_get_3 (Variables|Default|SetClass "/Game/Blueprints/Base/BP_AiBitcoin.BP_AiBitcoin_C"))
        (return _output_get_3)))))