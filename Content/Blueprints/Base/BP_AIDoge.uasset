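; Base AI enemy character, set to the DOGE type, that chases the player, attacks in melee and drops loot on death.
; A looping AIMoveTo pursues the player, while Tick pauses movement to play an attack montage within a randomized range.
; Capsule overlap with the player deals damage, independent of the montage.
; At zero health it updates the player's kill count, notifies the game mode, destroys itself and randomly spawns coins or health.
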(event OnComponentBeginOverlap(Capsule)
  (params (OverlappedComponent :type Primitive%20Component%20Object%20Reference) (OtherActor :type Actor%20Object%20Reference) (OtherComp :type Primitive%20Component%20Object%20Reference) (OtherBodyIndex :type Integer) (bFromSweep :type Boolean) (SweepResult :type Hit%20Result%20Structure%20%28by%20ref%29))
  (bind _asbp_player_dollar (Utilities|Casting|CastToBP_PlayerDollar OtherActor))
  (Utilities|IsValid _asbp_player_dollar
    (:Is%20Valid
      (CallFunction|DamageCharacter))))

(event EventBeginPlay
  (|CallParentFunction)
  (Variables|Default|SetCharacterType "NewEnumerator0")
  (AI|AIMoveTo self "0, 0, 0" (Game|GetPlayerCharacter 0) 5.0 false :!label _label
    (:OnSuccess
      _)
    (:OnFail
      _))
  (Utilities|FlowControl|Delay 0.2)
  (goto _label))

(event Collision|EventActorBeginOverlap
  (params (OtherActor :type Actor%20Object%20Reference)))

(event EventTick
  (params (DeltaSeconds :type Float%20%28single-precision%29))
  (if (CallFunction|CanAttack)
    (CallFunction|DeactivateAIMovement)
    (switch Utilities|FlowControl|Switch|SwitchonE_AnimMontages (Variables|Default|GetCharacterType)
      (:NewEnumerator0
        (Animation|Montage|PlayMontage (Variables|Character|GetMesh) "/Game/Zombie_Attack_Montage.Zombie_Attack_Montage"
          (:OnCompleted
            _)))
      (:NewEnumerator1
        (Animation|Montage|PlayMontage (Variables|Character|GetMesh) "/Game/Zombie_Attack_Montage.Zombie_Attack_Montage"
          (:OnCompleted
            _)))
      (:NewEnumerator2
        (Animation|Montage|PlayMontage (Variables|Character|GetMesh) "/Game/Zombie_Attack_Montage.Zombie_Attack_Montage"
          (:OnCompleted
            _))))
    (CallFunction|ActivateAIMovement)))

(event Game|Damage|EventAnyDamage
  (params (Damage :type Float%20%28single-precision%29) (DamageType :type Damage%20Type%20Object%20Reference) (InstigatedBy :type Controller%20Object%20Reference) (DamageCauser :type Actor%20Object%20Reference))
  (if (CallFunction|IsAlive)
    (bind _output_get (CallFunction|DescreamHealth Damage))
    (if (== 0.0 _output_get)
      (CallFunction|KillAi)
      (bind _output_get_2 (Variables|Default|SetPhysicalAnimation (Variables|Default|GetPhysicalAnimation)))
      (Components|Activation|Deactivate _output_get_2)
      (Actor|DestroyActor)
      (if (Math|Random|RandomBoolwithWeight 0.5)
        (CallFunction|SpawnMoney)
        (else
          (CallFunction|SpawnHealth))))))

(fn ConstructionScript
  (|CallParentFunction))

(fn IsWithinAttackRange
  (return (< (Transformation|GetDistanceTo (Game|GetPlayerCharacter 0)) (Math|Random|RandomFloatinRange (Variables|Default|GetAttackRange%20Min) (Variables|Default|GetAttackRange%20Max)))))

(fn IsAttacking
  (bind _mesh (Variables|Character|GetMesh))
  (bind _returnvalue (Components|SkeletalMesh|GetAnimInstance _mesh))
  (switch Utilities|FlowControl|Switch|SwitchonE_AnimMontages (Variables|Default|GetCharacterType)
    (:NewEnumerator0
      (return (Animation|Montage|MontageIsPlaying _returnvalue "/Game/Zombie_Attack_Montage.Zombie_Attack_Montage")))
    (:NewEnumerator1
      (return (Animation|Montage|MontageIsPlaying _returnvalue "/Game/Zombie_Attack_Montage.Zombie_Attack_Montage")))
    (:NewEnumerator2
      (return (Animation|Montage|MontageIsPlaying _returnvalue "/Game/Zombie_Attack_Montage.Zombie_Attack_Montage")))))

(fn DeactivateAIMovement
  (bind _charactermovement (Variables|Character|GetCharacterMovement))
  (Components|Movement|StopMovementImmediately _charactermovement)
  (Components|Activation|Deactivate _charactermovement))

(fn ActivateAIMovement
  (Components|Activation|Activate (Variables|Character|GetCharacterMovement) false))

(fn KillAi
  (Variables|Default|SetDead true)
  (CallFunction|DeactivateAIMovement)
  (Collision|SetActorEnableCollision false)
  (bind _asbp_player_dollar (Utilities|Casting|CastToBP_PlayerDollar (Game|GetPlayerCharacter 0)))
  (Default|IncreaseKill _asbp_player_dollar)
  (bind _asbp_main_game_mode_new (Utilities|Casting|CastToBP_MainGameModeNew (Game|GetGameMode)))
  (Default|RegisterEnemyDeath _asbp_main_game_mode_new self))

(fn DescreamHealth
  (params (Damage :type Float%20%28single-precision%29))
  (bind _output_get (Variables|Default|SetHealth (Math|Float|Clamp(Float) (- (Variables|Default|GetHealth) Damage) 0.0 (Variables|Default|GetMaxHealth))))
  (return _output_get))

(fn SpawnMoney
  (Game|SpawnActorfromClass "/Game/Blueprints/Actors/Drops/BP_Coins.BP_Coins_C" (Math|Transform|MakeTransform (Transformation|GetActorLocation) "0, 0, 0" "0.700000,0.700000,0.700000") "AlwaysSpawn" 0 0))

(fn SpawnHealth
  (Game|SpawnActorfromClass "/Game/Blueprints/Actors/Drops/BP_Health.BP_Health_C" (Math|Transform|MakeTransform (Transformation|GetActorLocation) "0, 0, 0" "0.700000,0.700000,0.700000") "Undefined" 0 0))

(fn CanAttack
  (return (Math|Boolean|ANDBoolean (CallFunction|IsWithinAttackRange) (not (CallFunction|IsAttacking)) (CallFunction|IsAlive))))

(fn DamageCharacter
  (bind _returnvalue (Game|GetPlayerCharacter 0))
  (Utilities|IsValid _returnvalue
    (:Is%20Valid
      (Game|Damage|ApplyDamage _returnvalue (Variables|Default|GetBase%20Damage) 0 0))))