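; BPC_Health is a component that stores a health value against a maximum and exposes functions to change and query it.
; Add applies an amount clamped between zero and MaxHealth, while GetHealth and GetPercent report the current value and fraction.
; IsDead tests whether the Health passed to it equals zero, and Remove, despite its name, resets Health to MaxHealth.
; The event graph holds no active logic.
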(event EventBeginPlay)

(event EventTick
  (params (DeltaSeconds :type Float%20%28single-precision%29)))

(fn GetHealth
  (return (Variables|Default|GetHealth)))

(fn Remove
  (Variables|Default|SetHealth (Variables|Default|GetMaxHealth)))

(fn IsDead
  (params (Health :type Float%20%28single-precision%29))
  (return (== Health 0.0)))

(fn Add
  (params (AddHealth :type Float%20%28single-precision%29))
  (Variables|Default|SetHealth (Math|Float|Clamp(Float) (+ (Variables|Default|GetHealth) AddHealth) 0.0 (Variables|Default|GetMaxHealth))))

(fn GetPercent
  (return (/ (Variables|Default|GetHealth) (Variables|Default|GetMaxHealth))))