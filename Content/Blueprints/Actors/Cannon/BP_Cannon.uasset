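; BP_Cannon is an automatic cannon that repeatedly fires BP_Projectile from its muzzle, starting at BeginPlay with no aiming or trigger.
; After a fire-rate delay, it spawns a scaled projectile at the muzzle's transform and restarts a timeline.
; The timeline animates the barrel along its local Y axis, and its Cannon Fire event track loops execution back to the delay for the next shot.
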(event EventBeginPlay
  (Utilities|FlowControl|Delay (Variables|CannonProjectile|GetCannonFireRate) :!label _label)
  (CallFunction|SpawnProjectile)
  (bind _barrellocation (Timeline|TL_CannonFIre PlayFromStart)
    (:Update
      (CallFunction|MoveCannonBarrel _barrellocation))
    (:Cannon%20Fire
      (goto _label))))

(event Collision|EventActorBeginOverlap
  (params (OtherActor :type Actor%20Object%20Reference)))

(event EventTick
  (params (DeltaSeconds :type Float%20%28single-precision%29)))

(fn ConstructionScript)

(fn SpawnProjectile
  (bind _cannonmuzzel (Variables|Default|GetCannonMuzzel))
  (Game|SpawnActorfromClass "/Game/Blueprints/Actors/Cannon/Projectile/BP_Projectile.BP_Projectile_C" (Math|Transform|MakeTransform (Transformation|GetWorldLocation _cannonmuzzel) (Transformation|GetWorldRotation _cannonmuzzel) (Math|Conversions|ToVector(Float) (Variables|CannonProjectile|GetProjectileScale))) "Undefined" 0 0))

(fn MoveCannonBarrel
  (params (CannonBarrelY%20Location :type Float%20%28single-precision%29))
  (Transformation|SetRelativeLocation (Variables|Default|GetCannonBarrel) (Math|Vector|MakeVector 0.0 CannonBarrelY%20Location 0.0) false false))