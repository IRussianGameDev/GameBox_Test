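; BP_DamageZone is a damage volume that repeatedly hurts a BP_PlayerDollar while it is inside.
; Actor begin overlap sets an InPlace flag, casts to the player, then loops through a short Delay, applying fixed damage and printing debug text.
; The Sphere's end overlap clears the flag for any valid actor, not only the player, which ends the loop at its next check.
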(event OnComponentEndOverlap(Sphere)
  (params (OverlappedComponent :type Primitive%20Component%20Object%20Reference) (OtherActor :type Actor%20Object%20Reference) (OtherComp :type Primitive%20Component%20Object%20Reference) (OtherBodyIndex :type Integer))
  (Utilities|IsValid OtherActor
    (:Is%20Valid
      (Development|PrintString "out")
      (Variables|Default|SetInPlace false))))

(event EventBeginPlay)

(event Collision|EventActorBeginOverlap
  (params (OtherActor :type Actor%20Object%20Reference))
  (Variables|Default|SetInPlace true)
  (bind _asbp_player_dollar (Utilities|Casting|CastToBP_PlayerDollar OtherActor))
  (bind _output_get (Variables|Default|SetAs%20BP%20Player%20Character _asbp_player_dollar))
  (if (Variables|Default|GetInPlace) :!label _label
    (Game|Damage|ApplyDamage _output_get 1e+01 0 0)
    (Development|PrintString "in" true true "(R=0.000000,G=1.000000,B=0.031292,A=1.000000)")
    (Utilities|FlowControl|Delay 0.2)
    (goto _label)))

(event EventTick
  (params (DeltaSeconds :type Float%20%28single-precision%29)))

(fn ConstructionScript)